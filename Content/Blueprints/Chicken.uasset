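; Player-controlled chicken that moves in short steps along world X and Y and can die.
; The Foward and Right axis inputs each offset the actor through a DoOnce reset after a brief Delay, throttling movement independently per axis.
; The Death event disables input, spawns a particle effect at the chicken, plays a sound at the world origin and hides the mesh without destroying the actor.
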(event Custom|Death
  ;[1 1 1] Death
  (Input|DisableInput 0)
  (Effects|SpawnEmitteratLocation 0 (Transformation|GetActorLocation))
  (Audio|PlaySoundatLocation 0 "0, 0, 0" "0, 0, 0" 1.0 1.0 0.0 0 0 0)
  (Rendering|SetVisibility (Variables|Default|GetChickenMesh) false false))

(event EventBeginPlay)

(event Collision|EventActorBeginOverlap
  (params (OtherActor :type Actor%20Object%20Reference)))

(event EventTick
  (params (DeltaSeconds :type Float%20%28single-precision%29)))

(event Input|AxisEvents|InputAxisFoward
  (params (AxisValue :type Float%20%28single-precision%29))
  (Utilities|FlowControl|DoOnce false :!label _label
    (:Completed
      (Transformation|AddActorWorldOffset (Math|Vector|MakeVector (* AxisValue 15.0) 0.0 0.0))
      (Utilities|FlowControl|Delay 0.1)
      (goto _label Reset))))

(event Input|AxisEvents|InputAxisRight
  (params (AxisValue :type Float%20%28single-precision%29))
  (Utilities|FlowControl|DoOnce false :!label _label
    (:Completed
      (Transformation|AddActorWorldOffset (Math|Vector|MakeVector 0.0 (* AxisValue 15.0) 0.0))
      (Utilities|FlowControl|Delay 0.1)
      (goto _label Reset))))

(fn ConstructionScript)