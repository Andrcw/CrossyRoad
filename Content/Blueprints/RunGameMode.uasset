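; RunGameMode is a game mode that lays out a randomized floor of blocks when play begins.
; On BeginPlay it calls AddFloorBlock in a short loop, spawning a random class from the Floor array at NextSpawnPoint each time.
; Each spawned block is cast to GrassBlock, and its attach transform becomes the next spawn point, chaining the pieces together.
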(event EventBeginPlay
  (for _index (range 0 5)
    (CallFunction|AddFloorBlock)))

(event EventTick
  (params (DeltaSeconds :type Float%20%28single-precision%29)))

(fn ConstructionScript)

(fn AddFloorBlock
  (bind _floor (Variables|Default|GetFloor))
  (bind _returnvalue (Game|SpawnActorfromClass (Utilities|Array|Get(acopy) _floor (Math|Random|RandomIntegerinRange 0 (Utilities|Array|LastIndex _floor))) (Variables|Default|GetNextSpawnPoint) "Undefined" 0 0))
  (bind _asgrass_block (Utilities|Casting|CastToGrassBlock _returnvalue))
  (bind _attachtransform (Default|GetAttachTransform _asgrass_block))
  (Variables|Default|SetNextSpawnPoint _attachtransform))